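; Base enemy character for melee combat against the hero, with empty events for attack, dodge, death and spotting animations.
; A state enum (patrol, fight, strafe, dead) is mirrored to the Blackboard, with first damage able to start combat and timers cycling strafe direction.
; Damage type scales health loss and selects stagger, and death halts AI logic.
; Tick turns it toward the player and eases a lagging damage bar; sphere traces deal hits.
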(fn ConstructionScript)

(fn LooktoPlayer
  ;[1 1 1] Look Player
  (Utilities|IsDeadCondition
    (:false
      (if (Variables|Bools|GetViewEnemy)
        (Transformation|SetActorRotation (Math|Rotator|MakeRotator 0.0 0.0 (.Yaw (Math|Rotator|BreakRotator (Math|Interpolation|RInterpTo (Transformation|GetActorRotation) (Math|Rotator|FindLookatRotation (Transformation|GetActorLocation self) (Transformation|GetActorLocation (Game|GetPlayerCharacter 0))) (Variables|Floats|GetDeltaTime) (Variables|Floats|GetInterpSpeed))))))))))

(fn ChangeState
  (params (ChangeState :type ChangeState_Enum%20Enum :default "NewEnumerator0"))
  (switch Utilities|FlowControl|Switch|SwitchonChangeState_Enum ChangeState
    (:NewEnumerator0
      (Variables|AI|SetChangeState_Enum "NewEnumerator0"))
    (:NewEnumerator1
      (Variables|AI|SetChangeState_Enum "NewEnumerator1"))
    (:NewEnumerator3
      (Variables|AI|SetChangeState_Enum "NewEnumerator3"))
    (:NewEnumerator2
      (Variables|AI|SetChangeState_Enum "NewEnumerator2"))))

(fn TraceCollision
  (bind _damagearrow (Variables|Default|GetDamageArrow))
  (bind _returnvalue (Transformation|GetWorldLocation _damagearrow))
  (bind _outhit (Collision|SphereTraceByChannel _returnvalue (+ _returnvalue (* (Math|Vector|GetForwardVector _damagearrow) 1.5e+02)) 5e+01 "TraceTypeQuery3" false 0 "None" true "(R=1.000000,G=0.000000,B=0.000000,A=1.000000)" "(R=0.000000,G=1.000000,B=0.000000,A=1.000000)" 1.0))
  (if (.bBlockingHit (Collision|BreakHitResult _outhit))
    (Game|Damage|ApplyDamage (.HitActor (Collision|BreakHitResult _outhit)) (Variables|AI|GetNormalDamageCause) 0 self "/Game/Blueprints/Hero/Notifys/NormalDamage_NTF.NormalDamage_NTF_C")
    (Utilities|PlayerIsBlock?)
    (Animation|PlayAnimMontage "/Game/GhostSamurai_Katana/Defense/Root/GhostSamurai_DefenseR_Rebound_1_Root_Montage.GhostSamurai_DefenseR_Rebound_1_Root_Montage" 1.0 "None")))

(fn WorldDirectionforStrafing
  (bind _returnvalue (Transformation|GetActorRightVector))
  (switch Utilities|FlowControl|Switch|SwitchonStrafingDirections_Enum (Variables|Enums|GetStrafingDirections_Enum)
    (:NewEnumerator0
      (Variables|Strafing|SetSD (* _returnvalue -1.0)))
    (:NewEnumerator1
      (Variables|Strafing|SetSD _returnvalue))
    (:NewEnumerator3
      (Variables|Strafing|SetSD (* (Transformation|GetActorForwardVector) -1.0))))
  (return (Variables|Strafing|GetSD)))

(fn GetWidgetProgressLifeBar
  (params (InputPin :type Float%20%28single-precision%29))
  (bind _health (Variables|AI|GetHealth))
  (bind _returnvalue (/ _health 1e+02))
  (bind _aswbp_enemy (Utilities|Casting|CastToWBP_Enemy (UserInterface|GetUserWidgetObject (Variables|Default|GetHealthWDG))))
  (Utilities|FlowControl|Sequence
    (:then_0
      (Progress|SetPercent (Variables|/Game/Blueprints/Enemy/Boss/Widgets/WBP_Enemy.WBP_Enemy_C|GetHealthBar _aswbp_enemy) _returnvalue))
    (:then_1
      (Progress|SetPercent (Variables|/Game/Blueprints/Enemy/Boss/Widgets/WBP_Enemy.WBP_Enemy_C|GetDamageBar _aswbp_enemy) (Math|Interpolation|FInterpTo (Variables|/Script/UMG.ProgressBar|GetPercent (Variables|/Game/Blueprints/Enemy/Boss/Widgets/WBP_Enemy.WBP_Enemy_C|GetDamageBar _aswbp_enemy)) _returnvalue InputPin 1.0)))))

(fn DodgeinCombat
  (bind _changestate_enum (Variables|AI|GetChangeState_Enum))
  (if (or (Utilities|Enum|Equal(Enum) _changestate_enum "NewEnumerator1") (Utilities|Enum|Equal(Enum) _changestate_enum "NewEnumerator3"))
    (Utilities|IsDeadCondition
      (:false
        (if (< (Transformation|GetDistanceTo (Variables|Refs|GetHero_Ref)) 3.5e+02)
          (switch int (Math|Random|RandomIntegerinRange 0 2)
            (:0
              (CallFunction|Dodge))))))))

(fn DamateType
  (if (== (Utilities|GetClass (Variables|Refs|GetDamageType)) "/Game/Blueprints/Hero/Notifys/NormalDamage_NTF.NormalDamage_NTF_C")
    (Variables|AI|SetHealth (- (Variables|AI|GetHealth) (Variables|AI|GetTakeDamage)))
    (CallFunction|CheckIsDeath :!label _label)
    (elif (== (Utilities|GetClass (Variables|Refs|GetDamageType)) "/Game/Blueprints/Hero/Notifys/StrongDamage_NTF.StrongDamage_NTF_C")
      (Variables|AI|SetHealth (- (Variables|AI|GetHealth) (* (Variables|AI|GetTakeDamage) 2.0)))
      (goto _label))))

(fn StaggerType
  (Utilities|IsDeadCondition
    (:false
      (if (== (Utilities|GetClass (Variables|Refs|GetDamageType)) "/Game/Blueprints/Hero/Notifys/NormalDamage_NTF.NormalDamage_NTF_C")
        (Animation|PlayAnimMontage "/Game/Blueprints/Enemy/Boss/Animations/Damage/Anim_CS_GH_F_01_Montage.Anim_CS_GH_F_01_Montage" 1.3 "None")
        (if (Utilities|Enum|Equal(Enum) (Variables|AI|GetChangeState_Enum) "NewEnumerator3")
          (CallFunction|ChangeState "NewEnumerator1")
          (CallFunction|RefreshBlackBoard))))))

(event Custom|NormalDeath
  ;[1 1 1] Death Animation
)

(event Custom|ResetDamage
  ;[1 1 1] Damage
  (Utilities|FlowControl|DoOnce false) ; enters at Reset
)

(event Custom|CooldownGetDamage
  ;[1 1 1] Cooldown Damage
  (Variables|Bools|SetIsInDamaged true)
  (Utilities|FlowControl|RetriggerableDelay 0.5)
  (Variables|Bools|SetIsInDamaged false))

(event Game|Damage|EventAnyDamage
  (params (Damage :type Float%20%28single-precision%29) (DamageType :type Damage%20Type%20Object%20Reference) (InstigatedBy :type Controller%20Object%20Reference) (DamageCauser :type Actor%20Object%20Reference))
  ;[1 1 1] Damage
  (Variables|Refs|SetDamageType DamageType)
  (Utilities|DamageCondition)
  (Utilities|FlowControl|Sequence
    (:then_0
      (Utilities|FlowControl|DoOnce false
        (:Completed
          (CallFunction|CooldownGetDamage)
          (CallFunction|DamateType)
          (CallFunction|StaggerType)
          (|FxDamage)
          (Utilities|FlowControl|Delay 0.1)
          (CallFunction|ResetDamage))))
    (:then_1
      (Utilities|FlowControl|DoOnce false
        (:Completed
          (CallFunction|IsFighting))))))

(event Custom|CheckIsDeath
  (if (<= (Variables|AI|GetHealth) 1.0)
    (Utilities|IsDeadCondition
      (:false
        (Variables|AI|SetIsDead true)
        (CallFunction|ChangeState "NewEnumerator2")
        (CallFunction|RefreshBlackBoard)
        (Components|Movement|StopMovementImmediately (Variables|Character|GetCharacterMovement))
        (AI|Logic|StopLogic (Variables|/Script/AIModule.AIController|GetBrainComponent (AI|GetAIController self)) "")
        (Development|SetHiddeninGame (Variables|Default|GetHealthWDG) true false)
        (Collision|SetCollisionEnabled (Variables|Collision|GetCapsuleComponent) "NoCollision")
        (CallFunction|NormalDeath)))))

(event Custom|StartFunctions
  (Utilities|Time|SetTimerbyFunctionName 0 "StrafingBehavior" (Math|Random|RandomFloatinRange 2.0 5.0) true)
  (Utilities|Time|SetTimerbyFunctionName 0 "GetWidgetProgressLifeBar" 0.1 true))

(event Custom|IsFighting
  ;[1 1 1] Is Begin Fighting
  (|BeginFightGraph))

(event Custom|ViewEnemyAnimation
  ;[1 1 1] View Enemy Event
)

(event EventBeginPlay
  ;[1 1 1] Begin Play
  (Variables|Default|SetTags (Utilities|Array|MakeArray "None"))
  (bind _ashero_bp (Utilities|Casting|CastToHero_BP (Game|GetPlayerCharacter 0)))
  (Variables|Refs|SetHero_Ref _ashero_bp)
  (bind _asenemy_abp (Utilities|Casting|CastToEnemy_ABP (Components|SkeletalMesh|GetAnimInstance (Variables|Character|GetMesh))))
  (Variables|Refs|SetAnimBP_Ref _asenemy_abp))

(event Custom|Dodge
  ;[1 1 1] Dodge Animations
)

(event EventTick
  (params (DeltaSeconds :type Float%20%28single-precision%29))
  (bind _output_get (Variables|Floats|SetDeltaTime DeltaSeconds))
  (CallFunction|LooktoPlayer)
  (CallFunction|GetWidgetProgressLifeBar _output_get))

(event Custom|CloseRange
  ;[1 1 1] Close Range
)

(event Custom|RefreshBlackBoard
  (bind _returnvalue (AI|GetBlackboard 0))
  (AI|Components|Blackboard|SetValueasEnum _returnvalue (Utilities|Name|MakeLiteralName "ChangeState") (Variables|AI|GetChangeState_Enum))
  (AI|Components|Blackboard|SetValueasBool _returnvalue (Utilities|Name|MakeLiteralName "StopMovement") (Variables|Bools|GetStopMovement))
  (AI|Components|Blackboard|SetValueasBool _returnvalue (Utilities|Name|MakeLiteralName "IsAttacking") (Variables|Bools|GetIsAttacking)))

(event Custom|StrafingBehavior
  ;[1 1 1] Strafing Behavior
  (switch Utilities|FlowControl|Switch|SwitchonStrafingDirections_Enum (Variables|Enums|GetStrafingDirections_Enum)
    (:NewEnumerator0
      (Variables|Enums|SetStrafingDirections_Enum "NewEnumerator1"))
    (:NewEnumerator1
      (Variables|Enums|SetStrafingDirections_Enum "NewEnumerator3"))
    (:NewEnumerator3
      (Variables|Enums|SetStrafingDirections_Enum "NewEnumerator0"))))

(event Custom|SetStrafingFunction
  ;[1 1 1] Strafing Behavior
  (Utilities|Time|SetTimerbyFunctionName 0 "StrafingBehavior" (Math|Random|RandomFloatinRange 1.5 3.0) true))