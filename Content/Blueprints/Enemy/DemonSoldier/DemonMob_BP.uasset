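; Demon soldier melee enemy extending a parent mob, with an optional dual-axe variant applied in the construction script.
; Random attack montages trace damage on notifies, then switch state and refresh the blackboard, with Tick driving strafe movement and animation.
; Hero attack-direction bindings set damage type and call combat dodging; random dodge montages briefly ignore one collision channel.
; Death plays an animation and notifies the player's ATS component.
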(fn ConstructionScript
  (switch Utilities|FlowControl|Switch|SwitchonDemonMobType_Enum (Variables|Default|GetMobType_Enum)
    (:NewEnumerator1
      (|DualAxeAttach))))

(event Custom|DodgeCooldown
  ;[1 1 1] Cooldown IsDodging
  (Collision|SetCollisionResponsetoChannel (Variables|Default|GetCapsuleComponent) "ECC_GameTraceChannel2" "ECR_Ignore")
  (Variables|Default|SetIsDodging true)
  (Utilities|FlowControl|RetriggerableDelay 1.0)
  (Variables|Default|SetIsDodging false)
  (Collision|SetCollisionResponsetoChannel (Variables|Default|GetCapsuleComponent) "ECC_GameTraceChannel2" "ECR_Block"))

(event EventDodge
  (Utilities|IsDodgeCondition
    (:else
      (CallFunction|DodgeCooldown)
      (switch int (Math|Random|RandomIntegerinRange 0 2)
        (:0
          (Animation|PlayAnimMontage "/Game/Blueprints/Hero/Animations/Dodge/Protector_Dodge_B_Montage.Protector_Dodge_B_Montage" 1.0 "None"))
        (:1
          (Animation|PlayAnimMontage "/Game/Blueprints/Hero/Animations/Dodge/Protector_Dodge_L_Montage.Protector_Dodge_L_Montage" 1.0 "None"))
        (:2
          (Animation|PlayAnimMontage "/Game/Blueprints/Hero/Animations/Dodge/Protector_Dodge_R_Montage.Protector_Dodge_R_Montage" 1.0 "None"))))))

(event Custom|AfterAttack
  ;[1 1 1] After Enemy Attack
  (Utilities|FlowControl|Delay (Math|Random|RandomFloatinRange 1.5 2.0))
  (Utilities|AfterAttackCondition
    (:else
      (switch int (Math|Random|RandomIntegerinRange 0 2)
        (:0
          (CallFunction|ChangeState "NewEnumerator1" :!label _label)
          (CallFunction|RefreshBlackBoard))
        (:1
          (goto _label))
        (:2
          (CallFunction|ChangeState "NewEnumerator3")
          (CallFunction|RefreshBlackBoard))))))

(event EventViewEnemyAnimation
  ;[1 1 1] See Player Anim
  (switch int (Math|Random|RandomIntegerinRange 0 1)
    (:0
      _)
    (:1
      _))
  (Animation|PlayAnimMontage "/Game/Blueprints/Enemy/DemonSoldier/Animations/TwoAxe/Protector_Attack14_Buff_Montage.Protector_Attack14_Buff_Montage" 1.0 "None"))

(event EventCloseRange
  ;[1 1 1] Close Range Combo
  (Utilities|CloseRangeCodition
    (:else
      (Variables|Default|SetIsAttacking true)
      (CallFunction|RefreshBlackBoard)
      (switch int (Math|Random|RandomIntegerinRange 0 3)
        (:0
          (bind _notifyname (Animation|Montage|PlayMontage (Variables|Character|GetMesh) "/Game/Blueprints/Enemy/DemonSoldier/Animations/TwoAxe/Montages/CCTwinSword_Attack05_Montage.CCTwinSword_Attack05_Montage" (Variables|Default|GetCombatSpeed))
            (:then
              (CallFunction|AfterAttack)
              (Utilities|FlowControl|Delay 2.0)
              (Variables|Default|SetIsAttacking false)
              (CallFunction|RefreshBlackBoard))
            (:OnNotifyBegin
              (if (Utilities|Name|Equal(Name) _notifyname "Damage")
                (CallFunction|TraceCollision)))))
        (:1
          (bind _notifyname_2 (Animation|Montage|PlayMontage (Variables|Character|GetMesh) "/Game/Blueprints/Enemy/DemonSoldier/Animations/TwoAxe/Montages/CCTwinSword_Attack06_Montage.CCTwinSword_Attack06_Montage" (Variables|Default|GetCombatSpeed))
            (:then
              (CallFunction|AfterAttack)
              (Utilities|FlowControl|Delay 2.0)
              (Variables|Default|SetIsAttacking false)
              (CallFunction|RefreshBlackBoard))
            (:OnNotifyBegin
              (if (Utilities|Name|Equal(Name) _notifyname_2 "Damage")
                (CallFunction|TraceCollision)))))
        (:2
          (bind _notifyname_3 (Animation|Montage|PlayMontage (Variables|Character|GetMesh) "/Game/Blueprints/Enemy/DemonSoldier/Animations/TwoAxe/Montages/CCTwinSword_Attack07_Montage.CCTwinSword_Attack07_Montage" (Variables|Default|GetCombatSpeed))
            (:then
              (CallFunction|AfterAttack)
              (Utilities|FlowControl|Delay 2.0)
              (Variables|Default|SetIsAttacking false)
              (CallFunction|RefreshBlackBoard))
            (:OnNotifyBegin
              (if (Utilities|Name|Equal(Name) _notifyname_3 "Damage")
                (CallFunction|TraceCollision)))))
        (:3
          (bind _notifyname_4 (Animation|Montage|PlayMontage (Variables|Character|GetMesh) "/Game/Blueprints/Enemy/DemonSoldier/Animations/TwoAxe/Montages/CCTwinSword_Attack08_Montage.CCTwinSword_Attack08_Montage" (Variables|Default|GetCombatSpeed))
            (:then
              (CallFunction|AfterAttack)
              (Utilities|FlowControl|Delay 2.0)
              (Variables|Default|SetIsAttacking false)
              (CallFunction|RefreshBlackBoard))
            (:OnNotifyBegin
              (if (Utilities|Name|Equal(Name) _notifyname_4 "Damage")
                (CallFunction|TraceCollision)))))))))

(event EventNormalDeath
  (Utilities|FlowControl|DoOnce false
    (:Completed
      (Components|Animation|PlayAnimation (Variables|Character|GetMesh) "/Game/Blueprints/Enemy/DemonSoldier/Animations/TwoAxe/CCTwinSword_Death.CCTwinSword_Death" false)
      (Collision|SetCollisionResponsetoChannel (Variables|Default|GetCapsuleComponent) "ECC_GameTraceChannel3" "ECR_Ignore")
      (Class|BPIRadar|NotifyDeath(Message) (Actor|GetComponentbyClass (Game|Player|GetPlayerPawn 0) "/Game/ActionTargetingSystem/Blueprints/ATS.ATS_C") self))))

(event EventTick
  (params (DeltaSeconds :type Float%20%28single-precision%29))
  (|CallParentFunction DeltaSeconds)
  (|StrafingGraph))

(event EventBeginPlay
  (|CallParentFunction)
  (CallFunction|StartFunctions)
  (|GetDamageDirections))

(event Custom|GetLeftAttack
  (Variables|Default|SetDamageType_Enum "NewEnumerator0")
  (CallFunction|DodgeinCombat))

(event Custom|GetRightAttack
  (Variables|Default|SetDamageType_Enum "NewEnumerator1")
  (CallFunction|DodgeinCombat))

(event Custom|GetFrontAttack
  (Variables|Default|SetDamageType_Enum "NewEnumerator3")
  (CallFunction|DodgeinCombat))