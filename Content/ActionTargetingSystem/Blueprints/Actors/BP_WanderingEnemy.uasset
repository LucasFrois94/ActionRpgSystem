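; BP_WanderingEnemy is an AI-controlled enemy character for the Action Targeting System that takes damage and ragdolls on death.
; Any damage reduces Health, and reaching zero triggers a one-time death sequence.
; Death enables mesh physics, makes the capsule ignore pawn, camera and targeting trace channels, notifies the player's ATS component and stops the AI brain logic.
; BeginPlay also resets the actor's tags.
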(event EventBeginPlay
  (Variables|Default|SetTags (Utilities|Array|MakeArray "None")))

(event Game|Damage|EventAnyDamage
  (params (Damage :type Float%20%28single-precision%29) (DamageType :type Damage%20Type%20Object%20Reference) (InstigatedBy :type Controller%20Object%20Reference) (DamageCauser :type Actor%20Object%20Reference))
  (bind _output_get (Variables|Default|SetHealth (- (Variables|Default|GetHealth) Damage)))
  (if (<= _output_get 0.0)
    (Utilities|FlowControl|DoOnce false
      (:Completed
        (Collision|SetCollisionEnabled (Variables|Character|GetMesh) "PhysicsOnly")
        (Physics|SetSimulatePhysics (Variables|Character|GetMesh) true)
        (Collision|SetCollisionResponsetoChannel (Variables|Collision|GetCapsuleComponent) "ECC_Pawn" "ECR_Ignore")
        (Collision|SetCollisionResponsetoChannel (Variables|Collision|GetCapsuleComponent) "ECC_Camera" "ECR_Ignore")
        ;[1 0 0] Set trace response to ignore and send interface message to ATS.
        (Collision|SetCollisionResponsetoChannel (Variables|Collision|GetCapsuleComponent) "ECC_GameTraceChannel1" "ECR_Ignore")
        (Default|NotifyDeath (Actor|GetComponentbyClass (Game|Player|GetPlayerPawn 0) "/Game/ActionTargetingSystem/Blueprints/ATS.ATS_C") self)
        (AI|Logic|StopLogic (Variables|/Script/AIModule.AIController|GetBrainComponent (AI|GetAIController self)) "Dead")))))

(fn ConstructionScript)