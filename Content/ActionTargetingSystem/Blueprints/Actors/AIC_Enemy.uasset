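; AI controller for enemies in the action targeting system that starts their behavior tree on possession.
; On possess it loads the enemy blackboard and runs the enemy behavior tree.
; It then stores the pawn's spawn position as the home location and a random navigable point within a wide radius around it as the initial target location.
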(event EventOnPossess
  (params (PossessedPawn :type Pawn%20Object%20Reference))
  (Class|AIController|UseBlackboard "/Game/ActionTargetingSystem/Blueprints/Actors/BB_Enemy.BB_Enemy")
  (AI|RunBehaviorTree "/Game/ActionTargetingSystem/Blueprints/Actors/BT_Enemy.BT_Enemy")
  (AI|Components|Blackboard|SetValueasVector (Variables|Default|GetBlackboard) (Variables|Default|GetHomeLocationKey) (Transformation|GetActorLocation (Pawn|GetControlledPawn)))
  (AI|Components|Blackboard|SetValueasVector (Variables|Default|GetBlackboard) (Variables|Default|GetTargetLocationKey) (.RandomLocation (Class|NavigationSystem|GetRandomPointinNavigableRadius (Transformation|GetActorLocation (Pawn|GetControlledPawn)) 5e+03))))

(fn ConstructionScript)